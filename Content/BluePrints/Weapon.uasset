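; Weapon Blueprint that provides automatic firing of projectiles while the trigger is held.
; PullTrigger fires immediately through a DoOnce gate, then starts a looping timer on Fire at an interval derived from RoundsPerSecond.
; ReleaseTrigger clears that timer and resets the gate, and each Fire call spawns the Projectile class at the ProjectileSpawnPoint transform.
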(event `PullTrigger`
  ;[1 1 1] Events that tell the weapon to fire when the player pulls the trigger
  (`/Engine/EditorBlueprintResources/StandardMacros.DoOnce` false :!label _label
    (:`Completed`
      (`self.Fire`)
      (`KismetSystemLibrary.K2_SetTimer` null "Fire" (/ 1.0 (`self.RoundsPerSecond`)) true))))

(event `ReleaseTrigger`
  ;[1 1 1] Events that tell the weapon to fire when the player pulls the trigger
  (`KismetSystemLibrary.K2_ClearTimer` null "Fire")
  (goto _label :!via `Reset`))

(event `Fire`
  ;[1 1 1] Events that tell the weapon to fire when the player pulls the trigger
  (`|SpawnActorFromClass` "/Game/BluePrints/Projectile.Projectile_C" (`SceneComponent.K2_GetComponentToWorld` (`self.ProjectileSpawnPoint`)) "Undefined" "OverrideRootScale" null null))

(fn `UserConstructionScript`)