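; Base character Blueprint for a twin-stick game, handling movement, aiming, shooting, health and death.
; On BeginPlay it spawns a weapon attached at GunTemp and saves its start transform to TwinStickMode for respawning.
; Move axes drive world-aligned movement, while look input past a dead zone sets control rotation and holds the weapon trigger.
; AffectHealth updates health; on death it disables input, waits, requests a respawn, then destroys character and weapon.
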(event `self.ReceiveBeginPlay`
  (bind _guntemp (`self.GunTemp`))
  ;[1 1 1] Spawn weapon and attach it to the hero character.
  (`|ExecutionSequence`
    (:`then_0`
      (bind _returnvalue (`|SpawnActorFromClass` "/Game/BluePrints/Weapon.Weapon_C" (`SceneComponent.K2_GetComponentToWorld` _guntemp) "Undefined" "OverrideRootScale" null null))
      (bind _output_get (set `self.Weapon` _returnvalue))
      (`self.K2_AttachToComponent` (`self.Weapon`) _guntemp "None" "SnapToTarget" "KeepRelative" "KeepWorld" true)
      (`self.K2_AttachToComponent` _output_get _guntemp "None" "SnapToTarget" "KeepRelative" "KeepWorld" true))
    (:`then_1`
      (bind _astwin_stick_mode (cast `/Game/BluePrints/TwinStickMode` (`GameplayStatics.GetGameMode`)))
      (bind _output_get_2 (set `self.GameMode` _astwin_stick_mode))
      (set `/Game/BluePrints/TwinStickMode.PlayerSpawnTransform` (`self.GetTransform`) _output_get_2))))

(event `InputAxis|Lookup`
  (params (AxisValue :type "Float (single-precision)"))
  (bind _weapon (`self.Weapon`))
  ;[1 1 1] Rotation
  (bind _returnvalue (`KismetMathLibrary.MakeVector` AxisValue (stale `InputAxis|LookRight` AxisValue)))
  (if (> (`KismetMathLibrary.VSize` _returnvalue) 0.25) :!label _label
    (`Controller.SetControlRotation` (`self.GetController`) (`KismetMathLibrary.Conv_VectorToRotator` _returnvalue))
    ;[1 1 1] Pull trigger when you rotate hero character
    (`/Game/BluePrints/Weapon.PullTrigger` _weapon)
    (else
      (`/Game/BluePrints/Weapon.ReleaseTrigger` _weapon))))

(event `InputAxis|LookRight`
  (params (AxisValue :type "Float (single-precision)"))
  ;[1 1 1] Rotation
  (goto _label))

(event `InputAxis|MoveUp`
  (params (AxisValue :type "Float (single-precision)"))
  ;[1 1 1] Movement
  (`self.AddMovementInput` (1.0 0.0 0.0) AxisValue))

(event `InputAxis|MoveRight`
  (params (AxisValue :type "Float (single-precision)"))
  ;[1 1 1] Movement
  (`self.AddMovementInput` (0.0 1.0 0.0) AxisValue))

(event `/Game/BluePrints/iDamagable.AffectHealth`
  (params (Delta :type "Float (single-precision)"))
  ;[1 1 1] Checks to see if the character is dead. If they are call respawn function
  (`self.CalculateHealth` Delta)
  (if (`self.IsDead`)
    (`self.DisableInput` null)
    (`KismetSystemLibrary.Delay` 3.0)
    (`/Game/BluePrints/TwinStickMode.RespawnPlayer` (`self.GameMode`))
    (`self.K2_DestroyActor` (`self.Weapon`))
    (`self.K2_DestroyActor` self)))

(fn `CalculateDead`
  ;[1 1 1] Checks to see if the character has died.
  (if (<= (`self.Health`) 0.0)
    (set `self.IsDead` true)
    (else
      (set `self.IsDead` false))))

(fn `CalculateHealth`
  (params (Delta :type "Float (double-precision)"))
  ;[1 1 1] Calculates Health
  (set `self.Health` (+ Delta (`self.Health`)))
  (`self.CalculateDead`))

(fn `UserConstructionScript`)