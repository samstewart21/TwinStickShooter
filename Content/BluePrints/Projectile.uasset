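; Projectile actor, apparently a laser shot, that damages non-friendly targets on overlap.
; Overlapped actors implementing IDamagable receive its Damage through AffectHealthMessage and the projectile is destroyed, unless they carry the Friendly tag, in which case it is unaffected.
; Any other actor triggers a 2D laser hit sound and a spark emitter at the projectile's transform before it destroys itself.
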(event `self.ReceiveActorBeginOverlap`
  (params (OtherActor :type "Actor Object Reference"))
  (bind (_returnvalue_location _returnvalue_rotation) (`KismetMathLibrary.BreakTransform` (`self.GetTransform`)))
  (if (`KismetSystemLibrary.DoesImplementInterface` OtherActor "/Game/BluePrints/iDamagable.iDamagable_C")
    (if (not (`self.ActorHasTag` OtherActor "Friendly"))
      (message `/Game/BluePrints/iDamagable.AffectHealth` OtherActor (`self.Damage`))
      (`self.K2_DestroyActor` :!label _label))
    (else
      (`GameplayStatics.PlaySound2D` "/Game/Audio/laser_hit.laser_hit" 1.0 1.0 0.0 null null)
      (`GameplayStatics.SpawnEmitterAtLocation` "/Game/StarterContent/Particles/LaserSparks.LaserSparks" _returnvalue_location _returnvalue_rotation)
      (goto _label))))

(fn `UserConstructionScript`)